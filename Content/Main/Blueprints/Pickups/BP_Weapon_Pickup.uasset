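; Weapon pickup actor that gives its configured weapon to the player on overlap.
; The construction script sets the pickup sprite flipbook from the WeaponToPickUp enum, covering Pistol and Rocket Launcher, with an empty flipbook for None.
; When a BP_Player begins overlapping, it passes that enum to the player's PickupWeapon and destroys itself.
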(event `self.ReceiveActorBeginOverlap`
  (params (OtherActor :type "Actor Object Reference"))
  (bind _asbp_player (cast `/Game/Main/Blueprints/Player/BP_Player` OtherActor))
  (`/Game/Main/Blueprints/Player/BP_Player.Pickup Weapon` _asbp_player (`self.WeaponToPickUp`))
  (`self.K2_DestroyActor`))

(fn `UserConstructionScript`
  (bind _pickup_sprite (`self.Pickup Sprite`))
  (switch `/Game/Main/Blueprints/ENUMS/ENUM_Weapon_List` (`self.WeaponToPickUp`)
    (:`NewEnumerator0`
      (`PaperFlipbookComponent.SetFlipbook` _pickup_sprite null))
    (:`NewEnumerator1`
      (`PaperFlipbookComponent.SetFlipbook` _pickup_sprite "/Game/Main/FlipBooks/Pickups/FB_Pistol_Pickup.FB_Pistol_Pickup"))
    (:`NewEnumerator2`
      (`PaperFlipbookComponent.SetFlipbook` _pickup_sprite "/Game/Main/FlipBooks/Pickups/FB_RocketLauncher_Pickup.FB_RocketLauncher_Pickup"))))