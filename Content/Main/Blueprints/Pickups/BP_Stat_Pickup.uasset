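; Health or armour stat pickup that comes in small and large sizes, displayed as a flipbook sprite.
; The construction script uses pickup type and size to set the sprite's flipbook, scale and gameplay tag.
; Two check functions read Ability System attributes to add or remove health-full and armour-full tags on the pickup's tag container.
; The event graph is empty, so overlap handling and calls to those checks are not in this graph.
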(fn `Full Armour Check`
  (params (`Ability System` :type "AbilitySystemComponent Object Reference"))
  (bind _pickup_tag (`self.Pickup Tag`))
  (if (== (`.ReturnValue` (`AbilitySystemBlueprintLibrary.GetFloatAttributeFromAbilitySystemComponent` `Ability System` (struct :`AttributeName` "Armour" :`Attribute` "/Script/FPS_Project.FPSAttributeSet:Armour" :`AttributeOwner` "/Script/CoreUObject.Class'\"/Script/FPS_Project.FPSAttributeSet\"'"))) 100.0)
    (`BlueprintGameplayTagLibrary.AddGameplayTag` _pickup_tag (struct :`TagName` "Player.Armour.Full"))
    (else
      (`BlueprintGameplayTagLibrary.RemoveGameplayTag` _pickup_tag (struct :`TagName` "Player.Armour.Full")))))

(fn `Full Health Check`
  (params (`Ability System` :type "AbilitySystemComponent Object Reference"))
  (bind _pickup_tag (`self.Pickup Tag`))
  (if (== (`.ReturnValue` (`AbilitySystemBlueprintLibrary.GetFloatAttributeFromAbilitySystemComponent` `Ability System` (struct :`AttributeName` "Health" :`Attribute` "/Script/FPS_Project.FPSAttributeSet:Health" :`AttributeOwner` "/Script/CoreUObject.Class'\"/Script/FPS_Project.FPSAttributeSet\"'"))) (`.ReturnValue` (`AbilitySystemBlueprintLibrary.GetFloatAttributeBaseFromAbilitySystemComponent` `Ability System` (struct :`AttributeName` "Health" :`Attribute` "/Script/FPS_Project.FPSAttributeSet:Health" :`AttributeOwner` "/Script/CoreUObject.Class'\"/Script/FPS_Project.FPSAttributeSet\"'"))))
    (`BlueprintGameplayTagLibrary.AddGameplayTag` _pickup_tag (struct :`TagName` "Player.Health.Full"))
    (else
      (`BlueprintGameplayTagLibrary.RemoveGameplayTag` _pickup_tag (struct :`TagName` "Player.Health.Full")))))

(fn `Set Stat Pickup Flipbook`
  (bind _pickup_sprite (`self.Pickup Sprite`))
  (bind _pickupsize (`self.PickupSize`))
  (bind _pickup_sprite_2 (`self.Pickup Sprite`))
  (switch `/Game/Main/Blueprints/ENUMS/ENUM_Pickup_Type` (`self.Pickup Type`)
    (:`NewEnumerator0`
      (`PaperFlipbookComponent.SetFlipbook` _pickup_sprite "/Game/Main/FlipBooks/Pickups/FB_ArmourPickup.FB_ArmourPickup")
      (switch `/Game/Main/Blueprints/ENUMS/ENUM_Pickup_Size` _pickupsize
        (:`NewEnumerator0`
          (`SceneComponent.SetRelativeScale3D` _pickup_sprite_2 (1.0 1.0 1.0))
          (set `self.Pickup Tag` (struct :`GameplayTags` (struct :`(TagName` "Pickup.Armour.Small")))))
        (:`NewEnumerator1`
          (`SceneComponent.SetRelativeScale3D` _pickup_sprite_2 (2.0 2.0 2.0))
          (set `self.Pickup Tag` (struct :`GameplayTags` (struct :`(TagName` "Pickup.Armour.Large")))))))
    (:`NewEnumerator1`
      (`PaperFlipbookComponent.SetFlipbook` _pickup_sprite "/Game/Main/FlipBooks/Pickups/FB_Health_Pickup.FB_Health_Pickup")
      (switch `/Game/Main/Blueprints/ENUMS/ENUM_Pickup_Size` _pickupsize
        (:`NewEnumerator0`
          (`SceneComponent.SetRelativeScale3D` _pickup_sprite_2 (1.0 1.0 1.0))
          (set `self.Pickup Tag` (struct :`GameplayTags` (struct :`(TagName` "Pickup.Health.Small")))))
        (:`NewEnumerator1`
          (`SceneComponent.SetRelativeScale3D` _pickup_sprite_2 (2.0 2.0 2.0))
          (set `self.Pickup Tag` (struct :`GameplayTags` (struct :`(TagName` "Pickup.Health.Large")))))))))

(fn `UserConstructionScript`
  (`parent.UserConstructionScript`)
  (`self.Set Stat Pickup Flipbook`))