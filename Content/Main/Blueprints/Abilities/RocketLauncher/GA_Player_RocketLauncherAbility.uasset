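; Player gameplay ability that fires the rocket launcher, spending special ammo per shot.
; FireWeapon checks an ability-system attribute is above zero, applies the ammo-spend effect, then tells the weapon to fire.
; Helpers lazily cache the player and the BP_RocketLauncher held in its weapon child actor.
; A camera line-trace helper, not called here, returns the hit actor or otherwise places a pooled object at the impact point.
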(event `self.Fire Weapon`
  (bind _player_rocketlauncher_weapon_component (`self.Player RocketLauncher Weapon Component`))
  ;[1 1 1] Fire Pistol
  (`self.Get Player`)
  (if (> (`.ReturnValue` (`AbilitySystemBlueprintLibrary.GetFloatAttributeFromAbilitySystemComponent` (`AbilitySystemBlueprintLibrary.GetAbilitySystemComponent` (`self.Player`)) (struct :`AttributeName` "SpecialAmmo" :`Attribute` "/Script/FPS_Project.FPSAttributeSet:SpecialAmmo" :`AttributeOwner` "/Script/CoreUObject.Class'\"/Script/FPS_Project.FPSAttributeSet\"'"))) 0.0)
    (`self.Get Weapon`)
    (`/Engine/EditorBlueprintResources/StandardMacros.IsValid` _player_rocketlauncher_weapon_component
      (:`Is Valid`
        (`self.BP_ApplyGameplayEffectToOwner` "/Game/Main/Blueprints/Abilities/RocketLauncher/GE_Player_SpecialAmmo_Spend.GE_Player_SpecialAmmo_Spend_C")
        (`/Game/Main/Blueprints/Weapons/BP_RocketLauncher.Fire Rocket Launcher` _player_rocketlauncher_weapon_component)))))

(fn `Get Line Trace`
  (returns (Actor :type "Actor Object Reference"))
  (bind _camera (`/Game/Main/Blueprints/Player/BP_Player.Camera` (`self.Player`)))
  (bind _returnvalue (`SceneComponent.K2_GetComponentLocation` _camera))
  (bind _outhit (`KismetSystemLibrary.LineTraceSingle` _returnvalue (+ _returnvalue (* (`KismetMathLibrary.GetForwardVector` (`SceneComponent.K2_GetComponentRotation` _camera)) (`self.Weapon Range`))) "TraceTypeQuery1"))
  (bind (_bblockinghit _binitialoverlap _time _distance _location _impactpoint _normal _impactnormal _physmat _hitactor) (`GameplayStatics.BreakHitResult` _outhit))
  (`/Engine/EditorBlueprintResources/StandardMacros.IsValid` _hitactor
    (:`Is Valid`
      (return _hitactor))
    (:`Is Not Valid`
      (bind _returnvalue_2 (`FPSObjectPool.SpawnPooledObject` (`/Game/Main/Blueprints/Player/BP_Player.FPSObjectPool` (`self.Player`))))
      (`Actor.K2_SetActorLocation` _returnvalue_2 _impactpoint false false)
      (`Actor.K2_SetActorRotation` _returnvalue_2 (`KismetMathLibrary.Conv_VectorToRotator` _impactnormal) false))))

(fn `Get Player`
  (bind _returnvalue_owneractor (break `GameplayAbilityActorInfo` (`self.GetActorInfo`)))
  (`/Engine/EditorBlueprintResources/StandardMacros.IsValid` (`self.Player`)
    (:`Is Valid`
      _)
    (:`Is Not Valid`
      (bind _asbp_player (cast `/Game/Main/Blueprints/Player/BP_Player` _returnvalue_owneractor))
      (set `self.Player` _asbp_player)))
  (return))

(fn `Get Weapon`
  (`/Engine/EditorBlueprintResources/StandardMacros.IsValid` (`self.Player RocketLauncher Weapon Component`)
    (:`Is Valid`
      _)
    (:`Is Not Valid`
      (bind _asbp_rocket_launcher (cast `/Game/Main/Blueprints/Weapons/BP_RocketLauncher` (`ChildActorComponent.ChildActor` (`/Game/Main/Blueprints/Player/BP_Player.Weapon` (`self.Player`)))))
      (set `self.Player RocketLauncher Weapon Component` _asbp_rocket_launcher)))
  (return))