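; BP_Rocket_Explosion is the visual effect actor for a rocket launcher explosion, drawn with a Paper2D flipbook.
; Each tick it billboards the flipbook toward player 0's camera on yaw only, with a 90-degree offset to keep the sprite upright and facing the view.
; On BeginPlay it waits for the flipbook's length, then destroys itself.
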(event `self.ReceiveBeginPlay`
  (`KismetSystemLibrary.Delay` (`PaperFlipbookComponent.GetFlipbookLength` (`self.Explosion Flipbook`)))
  (`self.K2_DestroyActor`))

(event `self.ReceiveTick`
  (params (DeltaSeconds :type "Float (single-precision)"))
  (bind _explosion_flipbook (`self.Explosion Flipbook`))
  (bind (_returnvalue_roll _returnvalue_pitch _returnvalue_yaw) (`KismetMathLibrary.BreakRotator` (`KismetMathLibrary.FindLookAtRotation` (`SceneComponent.K2_GetComponentLocation` _explosion_flipbook) (`PlayerCameraManager.GetCameraLocation` (`GameplayStatics.GetPlayerCameraManager` 0)))))
  (`SceneComponent.K2_SetWorldRotation` _explosion_flipbook (`KismetMathLibrary.MakeRotator` 0.0 0.0 (- _returnvalue_yaw 90.0)) false false))

(fn `UserConstructionScript`)