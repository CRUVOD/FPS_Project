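; Player gameplay ability that fires the shotgun as a hitscan spread of pellets.
; When a player attribute is above zero, it applies the bullet-spend effect, triggers the shotgun component and runs one randomly offset camera line trace per pellet.
; Each pellet hit on an FPSCharacter applies an effect, so hits stack per target.
; Traces without a valid hit actor place a pooled object at the impact point.
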(event `self.Fire Weapon`
  (bind _player_shotgun_weapon_component (`self.Player Shotgun Weapon Component`))
  ;[1 1 1] Fire Shotgun
  (`self.Get Player`)
  (if (> (`.ReturnValue` (`AbilitySystemBlueprintLibrary.GetFloatAttributeFromAbilitySystemComponent` (`AbilitySystemBlueprintLibrary.GetAbilitySystemComponent` (`self.Player`)) (struct :`AttributeName` "BulletAmmo" :`Attribute` "/Script/FPS_Project.FPSAttributeSet:BulletAmmo" :`AttributeOwner` "/Script/CoreUObject.Class'\"/Script/FPS_Project.FPSAttributeSet\"'"))) 0.0)
    (`self.Get Weapon`)
    (`/Engine/EditorBlueprintResources/StandardMacros.IsValid` _player_shotgun_weapon_component
      (:`Is Valid`
        (`self.BP_ApplyGameplayEffectToOwner` "/Game/Main/Blueprints/Abilities/Shotgun/GE_Player_Bullet_Spend2.GE_Player_Bullet_Spend2_C")
        (`/Game/Main/Blueprints/Weapons/BP_Shotgun.Fire Shotgun` _player_shotgun_weapon_component)
        (`self.Get Multi Line Traces`)
        (for _array_element (`self.HitActors`)
          (bind _asfpscharacter (cast `FPSCharacter` _array_element))
          (`self.Apply Effect` (`self.Player`) _asfpscharacter))))))

(fn `Get Line Trace With Random Spread`
  (returns (Actor :type "Actor Object Reference"))
  (bind _min_random_spread (`self.Min Random Spread`))
  (bind _max_random_spread (`self.Max Random Spread`))
  (bind _camera (`/Game/Main/Blueprints/Player/BP_Player.Camera` (`self.Player`)))
  (bind _returnvalue (`SceneComponent.K2_GetComponentLocation` _camera))
  (bind _outhit (`KismetSystemLibrary.LineTraceSingle` :`Start` _returnvalue :`End` (`KismetMathLibrary.MakeVector` (+ (.x (+ _returnvalue (* (`KismetMathLibrary.GetForwardVector` (`SceneComponent.K2_GetComponentRotation` _camera)) (`self.Weapon Range`)))) (`KismetMathLibrary.RandomFloatInRange` _min_random_spread _max_random_spread)) (+ (.y (+ _returnvalue (* (`KismetMathLibrary.GetForwardVector` (`SceneComponent.K2_GetComponentRotation` _camera)) (`self.Weapon Range`)))) (`KismetMathLibrary.RandomFloatInRange` _min_random_spread _max_random_spread)) (+ (`KismetMathLibrary.RandomFloatInRange` _min_random_spread _max_random_spread) (.z (+ _returnvalue (* (`KismetMathLibrary.GetForwardVector` (`SceneComponent.K2_GetComponentRotation` _camera)) (`self.Weapon Range`)))))) :`TraceChannel` "TraceTypeQuery1" :`DrawDebugType` "ForDuration" :`DrawTime` 4.0))
  (bind (_bblockinghit _binitialoverlap _time _distance _location _impactpoint _normal _impactnormal _physmat _hitactor) (`GameplayStatics.BreakHitResult` _outhit))
  (`/Engine/EditorBlueprintResources/StandardMacros.IsValid` _hitactor
    (:`Is Valid`
      (`KismetArrayLibrary.Array_Add` (`self.HitActors`) _hitactor)
      (return _hitactor))
    (:`Is Not Valid`
      (bind _returnvalue_2 (`FPSObjectPool.SpawnPooledObject` (`/Game/Main/Blueprints/Player/BP_Player.FPSObjectPool` (`self.Player`))))
      (`Actor.K2_SetActorLocation` _returnvalue_2 _impactpoint false false)
      (`Actor.K2_SetActorRotation` _returnvalue_2 (`KismetMathLibrary.Conv_VectorToRotator` _impactnormal) false))))

(fn `Get Multi Line Traces`
  (`KismetArrayLibrary.Array_Clear` (`self.HitActors`))
  (for _ (range (`self.Number of Pellets`))
    (`self.Get Line Trace With Random Spread`)))

(fn `Get Player`
  (bind _returnvalue_owneractor (break `GameplayAbilityActorInfo` (`self.GetActorInfo`)))
  (`/Engine/EditorBlueprintResources/StandardMacros.IsValid` (`self.Player`)
    (:`Is Valid`
      _)
    (:`Is Not Valid`
      (bind _asbp_player (cast `/Game/Main/Blueprints/Player/BP_Player` _returnvalue_owneractor))
      (set `self.Player` _asbp_player)))
  (return))

(fn `Get Weapon`
  (`/Engine/EditorBlueprintResources/StandardMacros.IsValid` (`self.Player Shotgun Weapon Component`)
    (:`Is Valid`
      _)
    (:`Is Not Valid`
      (bind _asbp_shotgun (cast `/Game/Main/Blueprints/Weapons/BP_Shotgun` (`ChildActorComponent.ChildActor` (`/Game/Main/Blueprints/Player/BP_Player.Weapon` (`self.Player`)))))
      (set `self.Player Shotgun Weapon Component` _asbp_shotgun)))
  (return))