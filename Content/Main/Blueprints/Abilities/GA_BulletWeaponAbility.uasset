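; Base gameplay ability for bullet weapons, leaving FireWeapon and Reset empty.
; On activation it commits, listens for WeaponEventTag, calls FireWeapon, then ends after the remaining cooldown time, which sets the fire rate.
; ApplyEffect sends that tag to the attacker with the target's data, so the listener applies WeaponEffect to the target.
; Ending the ability cleans up both wait tasks.
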(event `self.K2_ActivateAbility`
  ;[1 1 1] Activation
  (`self.K2_CommitAbility`)
  (`self.Wait For Event`)
  (`self.Fire Weapon`)
  ;[1 1 1] Ability Duration
  (bind _asynctaskproxy (`GameplayTask_WaitDelay.TaskWaitDelay` null (`self.GetCooldownTimeRemaining`))
    (:`then`
      (set `self.Fire Rate Delay Task` _asynctaskproxy))
    (:`OnFinish`
      (`self.K2_EndAbility`))))

(event `Wait For Event`
  ;[1 1 1] Wait For Gameplay Tag
  (bind (_asynctaskproxy _payload) (`AbilityTask_WaitGameplayEvent.WaitGameplayEvent` (`self.Weapon Event Tag`) null)
    (:`then`
      (set `self.Gameplay Event Wait Task` _asynctaskproxy))
    (:`EventReceived`
      (`self.BP_ApplyGameplayEffectToTarget` (`.TargetData` (break `GameplayEventData` _payload)) (`self.Weapon Effect`)))))

(event `Fire Weapon`
  ;[1 0 0.5701] To Override
)

(event `self.K2_OnEndAbility`
  (params (bWasCancelled :type Boolean))
  (bind _gameplay_event_wait_task (`self.Gameplay Event Wait Task`))
  (bind _fire_rate_delay_task (`self.Fire Rate Delay Task`))
  ;[1 1 1] End Ability Cleanup
  (`/Engine/EditorBlueprintResources/StandardMacros.IsValid` _gameplay_event_wait_task
    (:`Is Valid`
      (`GameplayTask.EndTask` _gameplay_event_wait_task))
    (:`Is Not Valid`
      _))
  (`/Engine/EditorBlueprintResources/StandardMacros.IsValid` _fire_rate_delay_task
    (:`Is Valid`
      (`GameplayTask.EndTask` _fire_rate_delay_task)
      (`self.Reset`))))

(fn `Apply Effect`
  (params (`Attacking Actor` :type "Actor Object Reference") (`Target Actor` :type "Actor Object Reference"))
  (`AbilitySystemBlueprintLibrary.SendGameplayEventToActor` `Attacking Actor` (`self.Weapon Event Tag`) (make `GameplayEventData` (struct) null `Target Actor` null null (struct) (struct) (struct) 0.0 (`AbilitySystemBlueprintLibrary.AbilityTargetDataFromActor` `Target Actor`))))

(fn `Reset`)