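; Player gameplay ability that fires the pistol as a camera-based hitscan shot.
; FireWeapon checks a positive ability-system attribute, spends a bullet via gameplay effect, then calls FirePistol on the lazily cached pistol.
; A visibility trace along camera forward applies an effect to any hit FPSCharacter.
; When the trace returns no valid actor, a pooled object is placed at the impact point, aligned to its normal.
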(event `self.Fire Weapon`
  (bind _player_pistol_weapon_component (`self.Player Pistol Weapon Component`))
  ;[1 1 1] Fire Pistol
  (`self.Get Player`)
  (if (> (`.ReturnValue` (`AbilitySystemBlueprintLibrary.GetFloatAttributeFromAbilitySystemComponent` (`AbilitySystemBlueprintLibrary.GetAbilitySystemComponent` (`self.Player`)) (struct :`AttributeName` "BulletAmmo" :`Attribute` "/Script/FPS_Project.FPSAttributeSet:BulletAmmo" :`AttributeOwner` "/Script/CoreUObject.Class'\"/Script/FPS_Project.FPSAttributeSet\"'"))) 0.0)
    (`self.Get Weapon`)
    (`/Engine/EditorBlueprintResources/StandardMacros.IsValid` _player_pistol_weapon_component
      (:`Is Valid`
        (`self.BP_ApplyGameplayEffectToOwner` "/Game/Main/Blueprints/Abilities/Pistol/GE_Player_Bullet_Spend.GE_Player_Bullet_Spend_C")
        (`/Game/Main/Blueprints/Weapons/BP_Pistol.Fire Pistol` _player_pistol_weapon_component)
        (bind _actor (`self.Get Line Trace`))
        (bind _asfpscharacter (cast `FPSCharacter` _actor))
        (`self.Apply Effect` (`self.Player`) _asfpscharacter)))))

(fn `Get Line Trace`
  (returns (Actor :type "Actor Object Reference"))
  (bind _camera (`/Game/Main/Blueprints/Player/BP_Player.Camera` (`self.Player`)))
  (bind _returnvalue (`SceneComponent.K2_GetComponentLocation` _camera))
  (bind _outhit (`KismetSystemLibrary.LineTraceSingle` _returnvalue (+ _returnvalue (* (`KismetMathLibrary.GetForwardVector` (`SceneComponent.K2_GetComponentRotation` _camera)) (`self.Weapon Range`))) "TraceTypeQuery1"))
  (bind (_bblockinghit _binitialoverlap _time _distance _location _impactpoint _normal _impactnormal _physmat _hitactor) (`GameplayStatics.BreakHitResult` _outhit))
  (`/Engine/EditorBlueprintResources/StandardMacros.IsValid` _hitactor
    (:`Is Valid`
      (return _hitactor))
    (:`Is Not Valid`
      (bind _returnvalue_2 (`FPSObjectPool.SpawnPooledObject` (`/Game/Main/Blueprints/Player/BP_Player.FPSObjectPool` (`self.Player`))))
      (`Actor.K2_SetActorLocation` _returnvalue_2 _impactpoint false false)
      (`Actor.K2_SetActorRotation` _returnvalue_2 (`KismetMathLibrary.Conv_VectorToRotator` _impactnormal) false))))

(fn `Get Player`
  (bind _returnvalue_owneractor (break `GameplayAbilityActorInfo` (`self.GetActorInfo`)))
  (`/Engine/EditorBlueprintResources/StandardMacros.IsValid` (`self.Player`)
    (:`Is Valid`
      _)
    (:`Is Not Valid`
      (bind _asbp_player (cast `/Game/Main/Blueprints/Player/BP_Player` _returnvalue_owneractor))
      (set `self.Player` _asbp_player)))
  (return))

(fn `Get Weapon`
  (`/Engine/EditorBlueprintResources/StandardMacros.IsValid` (`self.Player Pistol Weapon Component`)
    (:`Is Valid`
      _)
    (:`Is Not Valid`
      (bind _asbp_pistol (cast `/Game/Main/Blueprints/Weapons/BP_Pistol` (`ChildActorComponent.ChildActor` (`/Game/Main/Blueprints/Player/BP_Player.Weapon` (`self.Player`)))))
      (set `self.Player Pistol Weapon Component` _asbp_pistol)))
  (return))