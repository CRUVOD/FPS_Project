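; First-person shooter player character handling movement, mouse look, weapon inventory, pickups, interaction and the HUD.
; Weapon data comes from DT_FPSWeapons; equipping swaps a child actor's class and selects the gameplay tag used to fire.
; Firing and ammo gains activate Gameplay Abilities by tag, while UpdateUI reads attributes from the Ability System Component.
; Damage and pickups flash the HUD through timelines, and interaction messages the first overlapping actor implementing IPlayerInteractable.
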(event `self.ReceiveBeginPlay`
  ;[1 1 1] Initialization
  (bind _returnvalue (`|CreateWidget` "/Game/Main/Blueprints/Widgets/WBP_HUD.WBP_HUD_C"))
  (bind _output_get (set `self.HUD` _returnvalue))
  (`UserWidget.AddToViewport` _output_get 0)
  (`KismetSystemLibrary.Delay` 0.0)
  (`self.Update UI`)
  (`self.Initialise Weapon` "/Game/Main/Blueprints/Player/BP_PlayerWeaponBase.BP_PlayerWeaponBase_C")
  (`/Game/Main/Blueprints/Widgets/WBP_HUD.Switch Weapon` (`self.HUD`) "NewEnumerator0"))

(event `InputAxis|HorizontalMovement`
  (params (AxisValue :type "Float (single-precision)"))
  (bind (_returnvalue_roll _returnvalue_pitch _returnvalue_yaw) (`KismetMathLibrary.BreakRotator` (`self.GetControlRotation`)))
  ;[1 1 1] Movement
  (`self.AddMovementInput` (`KismetMathLibrary.GetRightVector` (`KismetMathLibrary.MakeRotator` 0.0 0.0 _returnvalue_yaw)) AxisValue))

(event `InputAction|Weapon Switch Slot 1`
  (params (Key :type "Key Structure"))
  ;[1 1 1] Weapon Switching
  (:`Pressed`
    (if (`self.Has Weapon` "NewEnumerator1")
      (bind _weapon_data (`self.Get Weapon From DataTable` "NewEnumerator1"))
      (`self.Equip Weapon` _weapon_data))))

(event `InputAxis|VerticalMovement`
  (params (AxisValue :type "Float (single-precision)"))
  (bind (_returnvalue_roll _returnvalue_pitch _returnvalue_yaw) (`KismetMathLibrary.BreakRotator` (`self.GetControlRotation`)))
  ;[1 1 1] Movement
  (`self.AddMovementInput` (`KismetMathLibrary.GetForwardVector` (`KismetMathLibrary.MakeRotator` 0.0 0.0 _returnvalue_yaw)) AxisValue))

(event `InputAction|Weapon Switch Slot 2`
  (params (Key :type "Key Structure"))
  ;[1 1 1] Weapon Switching
  (:`Pressed`
    (if (`self.Has Weapon` "NewEnumerator3")
      (bind _weapon_data (`self.Get Weapon From DataTable` "NewEnumerator3"))
      (`self.Equip Weapon` _weapon_data))))

(event `InputAxis|MouseLookHorizontal`
  (params (AxisValue :type "Float (single-precision)"))
  ;[1 1 1] MouseLook
  (`self.AddControllerYawInput` AxisValue))

(event `InputAction|Weapon Switch Slot 3`
  (params (Key :type "Key Structure"))
  ;[1 1 1] Weapon Switching
  (:`Pressed`
    (if (`self.Has Weapon` "NewEnumerator2")
      (bind _weapon_data (`self.Get Weapon From DataTable` "NewEnumerator2"))
      (`self.Equip Weapon` _weapon_data))))

(event `InputAxis|MouseLookVertical`
  (params (AxisValue :type "Float (single-precision)"))
  ;[1 1 1] MouseLook
  (`self.AddControllerPitchInput` AxisValue))

(event `InputAction|Interact`
  (params (Key :type "Key Structure"))
  (:`Pressed`
    (`self.Try Interact`)))

(event `Equip Weapon`
  (params (Weapon :type "/Game/Main/Blueprints/Structs/STRUCT_Weapon_Data Structure"))
  (bind _currentweapon_weaponname (break `/Game/Main/Blueprints/Structs/STRUCT_Weapon_Data` (`self.CurrentWeapon`)))
  (bind _currentweapon_weaponname_2 (break `/Game/Main/Blueprints/Structs/STRUCT_Weapon_Data` (`self.CurrentWeapon`)))
  ;[1 1 1] Equip Weapon
  (bind _output_get (set `self.CurrentWeapon` Weapon))
  (bind _weapon_actor (`self.Initialise Weapon` (`.Weapon_5_8B0CD33944FD3FA1AE19CEAE9F857F35` (break `/Game/Main/Blueprints/Structs/STRUCT_Weapon_Data` _output_get))))
  (`/Game/Main/Blueprints/Widgets/WBP_HUD.Switch Weapon` (`self.HUD`) _currentweapon_weaponname)
  (`self.Update UI`)
  (switch `/Game/Main/Blueprints/ENUMS/ENUM_Weapon_List` _currentweapon_weaponname_2
    (:`NewEnumerator0`
      (set `self.Weapon Fire Tag Container` (struct)))
    (:`NewEnumerator1`
      (set `self.Weapon Fire Tag Container` (struct :`GameplayTags` (struct :`(TagName` "Player.Weapon.Pistol.Fire")))))
    (:`NewEnumerator2`
      (set `self.Weapon Fire Tag Container` (struct :`GameplayTags` (struct :`(TagName` "Player.Weapon.RocketLauncher.Fire")))))
    (:`NewEnumerator3`
      (set `self.Weapon Fire Tag Container` (struct :`GameplayTags` (struct :`(TagName` "Player.Weapon.Shotgun.Fire")))))))

(event `self.ReceiveTick`
  (params (DeltaSeconds :type "Float (single-precision)"))
  ;[1 0 0] Not Used-Movement Weapon Bobbing Animation
)

(event `InputAction|Fire Weapon`
  (params (Key :type "Key Structure"))
  ;[1 1 1] Fire Weapon
  (:`Pressed`
    (`AbilitySystemComponent.TryActivateAbilitiesByTag` (`self.AbilitySystemComponent`) (`self.Weapon Fire Tag Container`) false)))

(event `self.Take Damage`
  (params (`Cue Data` :type "GameplayCueParameters Structure"))
  ;[1 1 1] Take Damage
  (`parent.Take Damage` `Cue Data`)
  (`self.Update UI`)
  (bind (_direction _alpha) (`Timeline|Damage Flash` :!via `PlayFromStart`)
    (:`Update`
      (`/Game/Main/Blueprints/Widgets/WBP_HUD.Set Flash Colour` (`self.HUD`) (struct :`R` 0.583333 :`G` 0.030382 :`B` 0.041736 :`A` 1.0) _alpha))))

(event `Item Pickup`
  ;[1 1 1] Item Pickup
  (`self.Update UI`)
  (bind (_direction _alpha) (`Timeline|Pickup Flash` :!via `PlayFromStart`)
    (:`Update`
      (`/Game/Main/Blueprints/Widgets/WBP_HUD.Set Flash Colour` (`self.HUD`) (struct :`G` 0.027964 :`B` 0.583333 :`A` 1.0) _alpha))))

(event `Pickup Weapon`
  (params (Weapon :type "/Game/Main/Blueprints/ENUMS/ENUM_Weapon_List Enum" :default "NewEnumerator0"))
  ;[1 1 1] Weapon Pickup
  (bind (_weapon_data _weapon_found) (`self.Get Weapon From DataTable` Weapon))
  (if _weapon_found
    (bind _output_get (set `self.Weapon To Pickup` _weapon_data))
    (if (`self.Has Weapon` (`.WeaponName_2_C9141B974E1D183AF527959D4E29F7B4` (break `/Game/Main/Blueprints/Structs/STRUCT_Weapon_Data` _output_get)))
      (bind (_weaponname _weapon _ammotype _ammoonpickupsize) (break `/Game/Main/Blueprints/Structs/STRUCT_Weapon_Data` _output_get))
      (`self.Add Ammo` _ammotype _ammoonpickupsize)
      (else
        (`self.Add Weapon`)))
    (else
      (`KismetSystemLibrary.PrintString` "Weapon does not exist in data_table"))))

(event `Add Ammo`
  (params (`Ammo Type` :type "/Game/Main/Blueprints/ENUMS/ENUM_Weapon_Ammo_List Enum" :default "NewEnumerator0") (`Ammo Size` :type "/Game/Main/Blueprints/ENUMS/ENUM_Pickup_Size Enum" :default "NewEnumerator0"))
  ;[1 1 1] Add Ammo
  (switch `/Game/Main/Blueprints/ENUMS/ENUM_Weapon_Ammo_List` `Ammo Type`
    (:`NewEnumerator1`
      (`self.Add Bullets` `Ammo Size`))
    (:`NewEnumerator2`
      (`self.Add SpecialAmmo` `Ammo Size`))))

(event `Add Weapon`
  (bind _weapon_to_pickup (`self.Weapon To Pickup`))
  (bind (_weaponname _weapon _ammotype _ammoonpickupsize) (break `/Game/Main/Blueprints/Structs/STRUCT_Weapon_Data` _weapon_to_pickup))
  ;[1 1 1] Add Weapon
  (`KismetArrayLibrary.Array_Add` (`self.Player Weapons`) _weapon_to_pickup)
  (`self.Equip Weapon` _weapon_to_pickup)
  (`self.Add Ammo` _ammotype _ammoonpickupsize))

(fn `Add Bullets`
  (params (`Ammo Size` :type "/Game/Main/Blueprints/ENUMS/ENUM_Pickup_Size Enum" :default "NewEnumerator0"))
  (if (not (>= (`.ReturnValue` (`AbilitySystemBlueprintLibrary.GetFloatAttributeFromAbilitySystemComponent` (`self.AbilitySystemComponent`) (struct :`AttributeName` "BulletAmmo" :`Attribute` "/Script/FPS_Project.FPSAttributeSet:BulletAmmo" :`AttributeOwner` "/Script/CoreUObject.Class'\"/Script/FPS_Project.FPSAttributeSet\"'"))) (`self.MaxBulletAmmo`)))
    (switch `/Game/Main/Blueprints/ENUMS/ENUM_Pickup_Size` `Ammo Size`
      (:`NewEnumerator0`
        (set `self.Ammo Gain Tag Container` (struct :`GameplayTags` (struct :`(TagName` "Pickup.Ammo.Bullets.Small"))))
        (`AbilitySystemComponent.TryActivateAbilitiesByTag` (`self.AbilitySystemComponent`) (`self.Ammo Gain Tag Container`) true)
        (`self.Item Pickup`)))))

(fn `Add SpecialAmmo`
  (params (`Ammo Size` :type "/Game/Main/Blueprints/ENUMS/ENUM_Pickup_Size Enum" :default "NewEnumerator0"))
  (if (not (>= (`.ReturnValue` (`AbilitySystemBlueprintLibrary.GetFloatAttributeFromAbilitySystemComponent` (`self.AbilitySystemComponent`) (struct :`AttributeName` "SpecialAmmo" :`Attribute` "/Script/FPS_Project.FPSAttributeSet:SpecialAmmo" :`AttributeOwner` "/Script/CoreUObject.Class'\"/Script/FPS_Project.FPSAttributeSet\"'"))) (`self.MaxSpecialAmmo`)))
    (switch `/Game/Main/Blueprints/ENUMS/ENUM_Pickup_Size` `Ammo Size`
      (:`NewEnumerator0`
        (set `self.Ammo Gain Tag Container` (struct :`GameplayTags` (struct :`(TagName` "Pickup.Ammo.SpecialAmmo.Small"))))
        (`AbilitySystemComponent.TryActivateAbilitiesByTag` (`self.AbilitySystemComponent`) (`self.Ammo Gain Tag Container`) true)
        (`self.Item Pickup`)))))

(fn `Get Weapon From DataTable`
  (params (Weapon :type "/Game/Main/Blueprints/ENUMS/ENUM_Weapon_List Enum" :default "NewEnumerator0"))
  (returns (`Weapon Data` :type "/Game/Main/Blueprints/Structs/STRUCT_Weapon_Data Structure") (`Weapon Found` :type Boolean))
  (locals (`Weapon Exists in Player Inventory` :type Boolean) (`Weapon to Equip` :type "/Game/Main/Blueprints/Structs/STRUCT_Weapon_Data Structure"))
  (bind _outrownames (`DataTableFunctionLibrary.GetDataTableRowNames` "/Game/Main/Blueprints/Weapons/DT_FPSWeapons.DT_FPSWeapons"))
  (for _array_element _outrownames
    (bind _returnvalue (`|GetDataTableRow` "/Game/Main/Blueprints/Weapons/DT_FPSWeapons.DT_FPSWeapons" _array_element)
      (:`then`
        (if (`|EnumEquality` Weapon (`.WeaponName_2_C9141B974E1D183AF527959D4E29F7B4` (break `/Game/Main/Blueprints/Structs/STRUCT_Weapon_Data` _returnvalue)))
          (set `local.Weapon Exists in Player Inventory` true)
          (set `local.Weapon to Equip` _returnvalue)
          (break)))))
  (return (`local.Weapon to Equip`) (`local.Weapon Exists in Player Inventory`)))

(fn `Has Weapon`
  (params (STRUCT_Weapon_Data :type "/Game/Main/Blueprints/ENUMS/ENUM_Weapon_List Enum" :default "NewEnumerator0"))
  (returns (`Has Weapon?` :type Boolean))
  (locals (`Has Weapon` :type Boolean))
  (for _array_element (`self.Player Weapons`)
    (if (`|EnumEquality` (`.WeaponName_2_C9141B974E1D183AF527959D4E29F7B4` (break `/Game/Main/Blueprints/Structs/STRUCT_Weapon_Data` _array_element)) STRUCT_Weapon_Data)
      (set `local.Has Weapon` true)
      (break)))
  (return (`local.Has Weapon`)))

(fn `Initialise Weapon`
  (params (`In Class` :type "/Game/Main/Blueprints/Player/BP_PlayerWeaponBase Class Reference"))
  (returns (`Weapon Actor` :type "Actor Object Reference"))
  (bind _weapon (`self.Weapon`))
  (bind _childactor (`ChildActorComponent.ChildActor` _weapon))
  (`ChildActorComponent.SetChildActorClass` _weapon `In Class`)
  (if (`KismetSystemLibrary.DoesImplementInterface` _childactor "/Game/Main/Blueprints/Interfaces/IPlayerWeapon.IPlayerWeapon_C")
    (message `/Game/Main/Blueprints/Interfaces/IPlayerWeapon.InitialiseWeapon` _childactor))
  (return _childactor))

(fn `Try Interact`
  (for _array_element (`self.GetOverlappingActors` null)
    (if (`KismetSystemLibrary.DoesImplementInterface` _array_element "/Game/Main/Blueprints/Interfaces/IPlayerInteractable.IPlayerInteractable_C")
      (message `/Game/Main/Blueprints/Interfaces/IPlayerInteractable.Interaction` _array_element)
      (`KismetSystemLibrary.PrintString` "Interactable Found")
      (break))))

(fn `Update UI`
  (bind _abilitysystemcomponent (`self.AbilitySystemComponent`))
  (bind _hud (`self.HUD`))
  (bind _currentammo (`/Game/Main/Blueprints/Widgets/WBP_HUD.CurrentAmmo` (`self.HUD`)))
  (`TextBlock.SetText` (`/Game/Main/Blueprints/Widgets/WBP_HUD.HealthValue` _hud) (`KismetTextLibrary.Conv_DoubleToText` (`.ReturnValue` (`AbilitySystemBlueprintLibrary.GetFloatAttributeFromAbilitySystemComponent` _abilitysystemcomponent (struct :`AttributeName` "Health" :`Attribute` "/Script/FPS_Project.FPSAttributeSet:Health" :`AttributeOwner` "/Script/CoreUObject.Class'\"/Script/FPS_Project.FPSAttributeSet\"'"))) "HalfToEven"))
  (`TextBlock.SetText` (`/Game/Main/Blueprints/Widgets/WBP_HUD.ArmourValue` _hud) (`KismetTextLibrary.Conv_DoubleToText` (`.ReturnValue` (`AbilitySystemBlueprintLibrary.GetFloatAttributeFromAbilitySystemComponent` _abilitysystemcomponent (struct :`AttributeName` "Armour" :`Attribute` "/Script/FPS_Project.FPSAttributeSet:Armour" :`AttributeOwner` "/Script/CoreUObject.Class'\"/Script/FPS_Project.FPSAttributeSet\"'"))) "HalfToEven"))
  (switch `/Game/Main/Blueprints/ENUMS/ENUM_Weapon_Ammo_List` (`.AmmoType_11_FD00A51A42A9017CF22BC9992FAB6FD9` (break `/Game/Main/Blueprints/Structs/STRUCT_Weapon_Data` (`self.CurrentWeapon`)))
    (:`NewEnumerator1`
      (`TextBlock.SetText` _currentammo (`KismetTextLibrary.Conv_DoubleToText` (`.ReturnValue` (`AbilitySystemBlueprintLibrary.GetFloatAttributeFromAbilitySystemComponent` (`self.AbilitySystemComponent`) (struct :`AttributeName` "BulletAmmo" :`Attribute` "/Script/FPS_Project.FPSAttributeSet:BulletAmmo" :`AttributeOwner` "/Script/CoreUObject.Class'\"/Script/FPS_Project.FPSAttributeSet\"'"))) "HalfToEven")))
    (:`NewEnumerator2`
      (`TextBlock.SetText` _currentammo (`KismetTextLibrary.Conv_DoubleToText` (`.ReturnValue` (`AbilitySystemBlueprintLibrary.GetFloatAttributeFromAbilitySystemComponent` (`self.AbilitySystemComponent`) (struct :`AttributeName` "SpecialAmmo" :`Attribute` "/Script/FPS_Project.FPSAttributeSet:SpecialAmmo" :`AttributeOwner` "/Script/CoreUObject.Class'\"/Script/FPS_Project.FPSAttributeSet\"'"))) "HalfToEven")))))

(fn `UserConstructionScript`)