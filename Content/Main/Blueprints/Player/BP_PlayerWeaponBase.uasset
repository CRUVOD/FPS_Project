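; BP_PlayerWeaponBase is a player weapon base that displays the weapon as a Paper2D flipbook sprite with movement bobbing.
; A SceneCaptureComponent2D is restricted to capturing only that flipbook, and InitialiseWeapon sets the flipbook and unhides it.
; WeaponBobbing plays the WeaponBob sequence while moving, otherwise stops it and interpolates the sprite back to its position cached at BeginPlay.
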(event `self.ReceiveBeginPlay`
  (`SceneCaptureComponent.ShowOnlyComponent` (`self.SceneCaptureComponent2D`) (`self.WeaponFlipBook`))
  (set `self.Weapon Sprite Position` (`SceneComponent.RelativeLocation` (`self.WeaponFlipBook`))))

(event `/Game/Main/Blueprints/Interfaces/IPlayerWeapon.InitialiseWeapon`
  (bind _weaponflipbook (`self.WeaponFlipBook`))
  (`PaperFlipbookComponent.SetFlipbook` _weaponflipbook null)
  (`SceneComponent.SetHiddenInGame` _weaponflipbook false false))

(event `Weapon Bobbing`
  (params (IsMoving :type Boolean) (DeltaTime :type "Float (double-precision)"))
  (bind _weaponflipbook (`self.WeaponFlipBook`))
  (bind _sequenceplayer (`ActorSequenceComponent.SequencePlayer` (`self.Weapon Bob`)))
  (if IsMoving
    (`MovieSceneSequencePlayer.Play` _sequenceplayer)
    (else
      (`MovieSceneSequencePlayer.Stop` _sequenceplayer)
      (`SceneComponent.K2_SetRelativeLocation` _weaponflipbook (`KismetMathLibrary.VInterpTo` (`SceneComponent.RelativeLocation` _weaponflipbook) (`self.Weapon Sprite Position`) DeltaTime 10.0) false false))))

(fn `UserConstructionScript`)