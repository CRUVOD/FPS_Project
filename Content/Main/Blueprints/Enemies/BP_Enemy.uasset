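; Base enemy character rendered as a Doom-style directional 2D sprite, driven by a behavior tree on its AI controller.
; Each tick it yaws the flipbook toward the camera, then picks one of eight walk or idle flipbooks from its angle and side relative to the player.
; Damage pauses that selection to play a hit flipbook; death stops the AI, disables capsule collision and plays dying then dead flipbooks.
; Melee and ranged attack events are empty.
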(event `self.ReceiveBeginPlay`
  (bind _asbp_fpsenemy_ai (cast `/Game/Main/Blueprints/Enemies/AI/BP_FPSEnemy_AI` (`self.GetController`)))
  (`AIController.RunBehaviorTree` _asbp_fpsenemy_ai (`self.Behaviour Tree`)))

(event `self.ReceiveTick`
  (params (DeltaSeconds :type "Float (single-precision)"))
  (`self.Sprite Face Player`
    (:`Out`
      (if (not (or (`self.Is Dead`) (`self.Pause Angle Calculations`)))
        (`self.Get Enemy Angle`
          (:`Out`
            (`self.Check If Walking`
              (:`Out`
                (`self.Calculate Flipbook`)))))))))

(event `self.Take Damage`
  (params (`Cue Data` :type "GameplayCueParameters Structure"))
  (bind _enemy_fb (`self.Enemy_FB`))
  ;[1 1 1] Take Damage
  (`parent.Take Damage` `Cue Data`)
  (if (not (`self.Is Dead`))
    (set `self.Pause Angle Calculations` true)
    (`PaperFlipbookComponent.SetFlipbook` _enemy_fb (`self.Damaged`))
    (`KismetSystemLibrary.Delay` (`PaperFlipbookComponent.GetFlipbookLength` _enemy_fb))
    (set `self.Pause Angle Calculations` false)))

(event `self.Kill Character`
  (bind _enemy_fb (`self.Enemy_FB`))
  ;[1 1 1] Death
  (`parent.Kill Character`)
  (bind _asbp_fpsenemy_ai (cast `/Game/Main/Blueprints/Enemies/AI/BP_FPSEnemy_AI` (`self.GetController`)))
  (`BrainComponent.StopLogic` (`AIController.BrainComponent` _asbp_fpsenemy_ai) "")
  (set `self.Is Dead` true)
  (`PrimitiveComponent.SetCollisionEnabled` (`self.CapsuleComponent`) "NoCollision")
  (`PaperFlipbookComponent.SetFlipbook` _enemy_fb (`self.Dying`))
  (`KismetSystemLibrary.Delay` (`PaperFlipbookComponent.GetFlipbookLength` _enemy_fb))
  (`PaperFlipbookComponent.SetFlipbook` (`self.Enemy_FB`) (`self.Dead`)))

(event `Melee Attack`)

(event `Ranged Attack`)

(fn `Set Flipbook`
  (params (Walking :type "PaperFlipbook Object Reference") (Idle :type "PaperFlipbook Object Reference"))
  (bind _enemy_fb (`self.Enemy_FB`))
  (if (`self.Is Walking`)
    (`PaperFlipbookComponent.SetFlipbook` _enemy_fb Walking)
    (else
      (`PaperFlipbookComponent.SetFlipbook` _enemy_fb Idle))))

(fn `UserConstructionScript`)